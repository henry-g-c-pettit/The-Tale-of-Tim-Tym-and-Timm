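; EnemyController is an AI controller for enemy pawns that wraps behavior tree startup and Blackboard writes.
; On possession it stores the pawn, and RunBT starts the AIBT tree and sets that pawn as SelfActor.
; Two update functions write the target actor and line-of-sight flag to the Blackboard.
; Nothing in this Blueprint calls these three functions.
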(event EventBeginPlay)

(event EventTick
  (params (DeltaSeconds :type Float%20%28single-precision%29)))

(event EventPossess
  (params (PossessedPawn :type Pawn%20Object%20Reference))
  (Variables|Default|SetPossessedPawn PossessedPawn))

(fn ConstructionScript)

(fn UpdateTargetActorKey
  (params (TargetActor :type Actor%20Object%20Reference))
  (AI|Components|Blackboard|SetValueasObject (Variables|Default|GetBlackboard) (Variables|Default|GetTargetActor) TargetActor))

(fn UpdateHasLineOfSightKey
  (params (HasLineOfSight :type Boolean))
  (AI|Components|Blackboard|SetValueasBool (Variables|Default|GetBlackboard) (Variables|Default|GetHasLineOfSIght) HasLineOfSight))

(fn RunBT
  (AI|RunBehaviorTree (Variables|Default|GetAI_BT))
  (AI|Components|Blackboard|SetValueasObject (Variables|Default|GetBlackboard) (Variables|Default|GetSelfActor) (Variables|Default|GetPossessedPawn)))