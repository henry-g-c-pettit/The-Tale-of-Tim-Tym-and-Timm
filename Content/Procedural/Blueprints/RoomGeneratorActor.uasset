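; Procedural dungeon-style room generator actor that builds a random floor layout on BeginPlay.
; It places random, non-overlapping rooms on a square grid until hitting a room or failure limit, then spawns instanced floor tiles.
; It links all room pairs by distance and greedily picks shortest edges for an approximate spanning tree, skipping those with both rooms already connected.
; Corridor generation along those edges is unfinished: its bounds check is disconnected and spawns nothing.
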(event EventBeginPlay
  (CallFunction|GenerateAllRooms)
  (bind _room_centers (CallFunction|FindCenter))
  (bind _edges (CallFunction|CreateEdges _room_centers))
  (bind _mst (CallFunction|MST _edges))
  (CallFunction|GenerateAllCorridors _mst)
  (CallFunction|CreateRooms))

(fn ConstructionScript)

(fn GenerateRoom
  ;[1 1 1] Create X*Y Sized Room
  (bind _output_get (LocalVariables|SetSize (Math|Vector|MakeVector (Math|Conversions|ToFloat(Integer) (Math|Random|RandomIntegerinRange (Variables|Default|GetMinRoomSize) (Variables|Default|GetMaxRoomSize))) (Math|Conversions|ToFloat(Integer) (Math|Random|RandomIntegerinRange (Variables|Default|GetMinRoomSize) (Variables|Default|GetMaxRoomSize))) 0.0)))
  ;[1 1 1] Randomise Room Position within Map Size Grid
  (bind _output_get_2 (LocalVariables|SetPosition (Math|Vector|MakeVector (Math|Conversions|ToFloat(Integer) (Math|Random|RandomIntegerinRange 0 (- (Variables|Default|GetMaze%20Size) (Math|Float|Truncate (.X (Math|Vector|BreakVector _output_get)))))) (Math|Conversions|ToFloat(Integer) (Math|Random|RandomIntegerinRange 0 (- (Variables|Default|GetMaze%20Size) (Math|Float|Truncate (.Y (Math|Vector|BreakVector _output_get)))))) 0.0)))
  (return _output_get_2 (LocalVariables|GetSize)))

(fn GenerateAllRooms
  ;[1 1 1] Create Rooms as long as there is space
  (while (and (< (LocalVariables|GetCurrentRooms) (Variables|Default|GetMaxRooms)) (< (LocalVariables|GetFailCounter) (LocalVariables|GetMaxF)))
    (bind (_roomposition _roomsize) (CallFunction|GenerateRoom))
    ;[1 1 1] No Overlap - Room is Valid add to array
    (bind _overlap (CallFunction|CheckOverlap _roomposition _roomsize))
    (if _overlap
      (Math|Integer|IncrementInt (LocalVariables|GetFailCounter))
      (else
        (Utilities|Array|Add (Variables|Default|GetRoomPositions) _roomposition)
        (Utilities|Array|Add (Variables|Default|GetRoomSizes) _roomsize)
        (Math|Integer|IncrementInt (LocalVariables|GetCurrentRooms)
          (:%20%20
            (LocalVariables|SetFailCounter 0))))))
  (return))

(fn CheckOverlap
  (params (RoomPosition :type Vector) (RoomSize :type Vector))
  (bind (_x _y) (Math|Vector|BreakVector RoomPosition))
  (bind (_x_2 _y_2) (Math|Vector|BreakVector RoomSize))
  ;[1 1 1] Check Overlap - Overlap Boolean Checkers not very clean but works for now
  ;;[1 1 1] Set Variables for New Room
  (LocalVariables|SetNewRoomXPos _x)
  (LocalVariables|SetNewRoomYPos _y)
  (LocalVariables|SetNewRoomXSize (+ _x _x_2))
  (LocalVariables|SetNewRoomYSize (+ _y _y_2))
  ;;[1 1 1] Set Variables for Old Room(s) - For Each Loop
  (for (_array_element _array_index) (Variables|Default|GetRoomPositions)
    (bind _output_get (LocalVariables|SetOldRoomXPos (.X (Math|Vector|BreakVector _array_element))))
    (bind _output_get_2 (LocalVariables|SetOldRoomYPos (.Y (Math|Vector|BreakVector _array_element))))
    (LocalVariables|SetOldRoomXSize (+ _output_get (.X (Math|Vector|BreakVector (Utilities|Array|Get(acopy) (Variables|Default|GetRoomSizes) _array_index)))))
    (LocalVariables|SetOldRoomYSize (+ _output_get_2 (.Y (Math|Vector|BreakVector (Utilities|Array|Get(acopy) (Variables|Default|GetRoomSizes) _array_index)))))
    (if (Math|Boolean|ORBoolean (Math|Boolean|ANDBoolean (<= (LocalVariables|GetNewRoomXPos) (LocalVariables|GetOldRoomXPos)) (<= (LocalVariables|GetNewRoomYPos) (LocalVariables|GetOldRoomYPos)) (>= (LocalVariables|GetNewRoomXSize) (LocalVariables|GetOldRoomXPos)) (>= (LocalVariables|GetNewRoomYSize) (LocalVariables|GetOldRoomYPos))) (Math|Boolean|ANDBoolean (<= (LocalVariables|GetOldRoomXPos) (LocalVariables|GetNewRoomXPos)) (<= (LocalVariables|GetOldRoomYPos) (LocalVariables|GetNewRoomYPos)) (>= (LocalVariables|GetOldRoomXSize) (LocalVariables|GetNewRoomXPos)) (>= (LocalVariables|GetOldRoomYSize) (LocalVariables|GetNewRoomYPos))) (Math|Boolean|ANDBoolean (>= (LocalVariables|GetOldRoomXPos) (LocalVariables|GetNewRoomXPos)) (<= (LocalVariables|GetOldRoomXPos) (LocalVariables|GetNewRoomXSize)) (>= (+ (LocalVariables|GetOldRoomYSize) (Variables|Default|GetOverlapTest)) (LocalVariables|GetNewRoomYPos))) (Math|Boolean|ANDBoolean (>= (LocalVariables|GetNewRoomXPos) (LocalVariables|GetOldRoomXPos)) (<= (LocalVariables|GetNewRoomXPos) (LocalVariables|GetOldRoomXSize)) (>= (+ (LocalVariables|GetNewRoomYSize) (Variables|Default|GetOverlapTest)) (LocalVariables|GetOldRoomYPos))) (Math|Boolean|ANDBoolean (>= (LocalVariables|GetOldRoomYPos) (LocalVariables|GetNewRoomYPos)) (<= (LocalVariables|GetOldRoomYPos) (LocalVariables|GetNewRoomYSize)) (>= (+ (LocalVariables|GetOldRoomXSize) (Variables|Default|GetOverlapTest)) (LocalVariables|GetNewRoomXPos))) (Math|Boolean|ANDBoolean (>= (LocalVariables|GetNewRoomYPos) (LocalVariables|GetOldRoomYPos)) (<= (LocalVariables|GetNewRoomYPos) (LocalVariables|GetOldRoomYSize)) (>= (+ (LocalVariables|GetNewRoomXSize) (Variables|Default|GetOverlapTest)) (LocalVariables|GetOldRoomXPos))))
      (return true)))
  (return false))

(fn FindCenter
  ;[1 1 1] Find Center Points of each Room
  (for (_array_element _array_index) (Variables|Default|GetRoomPositions)
    (Utilities|Array|Add (LocalVariables|GetCenterPoints) (Math|Vector|MakeVector (/ (+ (.X (Math|Vector|BreakVector _array_element)) (.X (Math|Vector|BreakVector (Utilities|Array|Get(acopy) (Variables|Default|GetRoomSizes) _array_index)))) 2.0) (/ (+ (.Y (Math|Vector|BreakVector _array_element)) (.Y (Math|Vector|BreakVector (Utilities|Array|Get(acopy) (Variables|Default|GetRoomSizes) _array_index)))) 2.0) (Math|Conversions|ToFloat(Integer) _array_index))))
  (return (LocalVariables|GetCenterPoints)))

(fn CreateEdges
  (params (RoomsCenters :type Array%20of%20Vectors))
  ;[1 1 1] Create all edges between Rooms
  (for _array_element RoomsCenters
    (for _array_element_2 RoomsCenters
      (if (Math|Vector|NotEqual(Vector) _array_element_2 _array_element 0.1)
        (Utilities|Array|Add (LocalVariables|GetRoomsEdges) (Math|Vector|MakeVector (.Z (Math|Vector|BreakVector _array_element)) (.Z (Math|Vector|BreakVector _array_element_2)) (Math|Float|Sqrt (+ (Math|Float|Power (- (.X (Math|Vector|BreakVector _array_element)) (.X (Math|Vector|BreakVector _array_element_2))) 2.0) (Math|Float|Power (- (.Y (Math|Vector|BreakVector _array_element)) (.Y (Math|Vector|BreakVector _array_element_2))) 2.0))))))))
  (return (LocalVariables|GetRoomsEdges)))

(fn MST
  (params (Edges :type Array%20of%20Vectors))
  (bind _connectedrooms (LocalVariables|GetConnectedRooms))
  (bind _connectedrooms_2 (LocalVariables|GetConnectedRooms))
  ;[1 1 1] Loop while Edges remain or not all Rooms connected
  (bind _output_get (LocalVariables|SetRemainingEdges Edges))
  (while (or (!= (Utilities|Array|Length (LocalVariables|GetConnectedRooms)) (Utilities|Array|Length (Variables|Default|GetRoomPositions))) (> (Utilities|Array|Length (LocalVariables|GetRemainingEdges)) 0))
    ;[1 1 1] Add Minimum Edge if Nodes aren't Connected
    (bind (_minimum_edge _newedges) (CallFunction|MinimumEdge _output_get))
    (bind _output_get_2 (LocalVariables|SetMinEdge _minimum_edge))
    (LocalVariables|SetRemainingEdges _newedges)
    (LocalVariables|SetFirstRoomIndex (.X (Math|Vector|BreakVector _output_get_2)))
    (LocalVariables|SetSecondRoomIndex (.Y (Math|Vector|BreakVector _output_get_2)))
    (if (not (and (Utilities|Array|ContainsItem _connectedrooms_2 (LocalVariables|GetFirstRoomIndex)) (Utilities|Array|ContainsItem _connectedrooms_2 (LocalVariables|GetSecondRoomIndex))))
      (Utilities|FlowControl|Sequence
        (:then_0
          (if (not (Utilities|Array|ContainsItem _connectedrooms_2 (LocalVariables|GetFirstRoomIndex)))
            (Utilities|Array|Add _connectedrooms (LocalVariables|GetFirstRoomIndex))))
        (:then_1
          (if (not (Utilities|Array|ContainsItem _connectedrooms_2 (LocalVariables|GetSecondRoomIndex)))
            (Utilities|Array|Add _connectedrooms (LocalVariables|GetSecondRoomIndex))))
        (:then_2
          (Utilities|Array|Add (LocalVariables|GetMinimumSpanTree) (LocalVariables|GetMinEdge))))))
  (return (LocalVariables|GetMinimumSpanTree)))

(fn MinimumEdge
  (params (Edges :type Array%20of%20Vectors))
  ;[1 1 1] Find the Shortest Edge
  (bind _output_get (LocalVariables|SetTempEdges Edges))
  (for _array_element _output_get
    (if (LocalVariables|GetFirstLoop)
      (LocalVariables|SetMinEdge _array_element)
      (LocalVariables|SetFirstLoop false)
      (elif (< (.Z (Math|Vector|BreakVector _array_element)) (.Z (Math|Vector|BreakVector (LocalVariables|GetMinEdge))))
        (LocalVariables|SetMinEdge _array_element))))
  (Utilities|Array|RemoveItem (LocalVariables|GetTempEdges) (LocalVariables|GetMinEdge))
  (return (LocalVariables|GetMinEdge) (LocalVariables|GetTempEdges)))

(fn GenerateCorridor
  (params (APos :type Vector) (ASize :type Vector) (BPos :type Vector) (BSize :type Vector))
  ;[1 1 1] Define Corners of Each Room as Local Variables
  (bind _output_get (LocalVariables|SetFirstPosition APos))
  (bind _output_get_2 (LocalVariables|SetFirstSize ASize))
  (bind _output_get_3 (LocalVariables|SetSecondPos BPos)))

(fn CreateRooms
  (for (_array_element _array_index) (Variables|Default|GetRoomPositions)
    (CallFunction|SpawnFloor _array_element (Utilities|Array|Get(acopy) (Variables|Default|GetRoomSizes) _array_index)))
  (return))

(fn SpawnFloor
  (params (Pos :type Vector) (Size :type Vector))
  (bind (_x _y) (Math|Vector|BreakVector Size))
  (bind _tilesize (Variables|Default|GetTileSize))
  (for _index (range 0 (Math|Float|Truncate _x))
    (for _index_2 (range 0 (Math|Float|Truncate _y))
      (Components|InstancedStaticMesh|AddInstance (Variables|Default|GetRoomFloor) (Math|Conversions|ToTransform(Vector) (+ (Math|Vector|MakeVector (* _index _tilesize) (* _index_2 _tilesize) 0.0) (* Pos _tilesize))))))
  (return))

(fn GenerateAllCorridors
  (params (Edges :type Array%20of%20Vectors))
  (bind _roompositions (Variables|Default|GetRoomPositions))
  (bind _roomsizes (Variables|Default|GetRoomSizes))
  (for _array_element Edges
    (CallFunction|GenerateCorridor (Utilities|Array|Get(acopy) _roompositions (Math|Float|Truncate (.X (Math|Vector|BreakVector _array_element)))) (Utilities|Array|Get(acopy) _roomsizes (Math|Float|Truncate (.X (Math|Vector|BreakVector _array_element)))) (Utilities|Array|Get(acopy) _roompositions (Math|Float|Truncate (.Y (Math|Vector|BreakVector _array_element)))) (Utilities|Array|Get(acopy) _roomsizes (Math|Float|Truncate (.Y (Math|Vector|BreakVector _array_element))))))
  (return))

(fn SpawnCorridorTest
  (params (Pos :type Vector) (Size :type Vector))
  (bind (_x _y) (Math|Vector|BreakVector Size))
  (bind _tilesize (Variables|Default|GetTileSize))
  (for _index (range 0 (Math|Float|Truncate _x))
    (for _index_2 (range 0 (Math|Float|Truncate _y))
      (Components|InstancedStaticMesh|AddInstance (Variables|Default|GetCorridorFloor) (Math|Conversions|ToTransform(Vector) (+ (Math|Vector|MakeVector (* _index _tilesize) (* _index_2 _tilesize) 25.0) (* Pos _tilesize))))))
  (return))