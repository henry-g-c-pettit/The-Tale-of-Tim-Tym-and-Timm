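; Procedural room layout generator that fills a square map grid with randomly sized and positioned rectangular rooms on BeginPlay, storing positions and sizes without spawning geometry.
; GenerateAllRooms rejection-samples candidates through GenerateRoom and CheckOverlap until it reaches the room cap or a limit of consecutive failures.
; FindCenter, meant to compute room center points with the room index in Z, is never called, and KruskalMSTCorridors is an empty stub.
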(event EventBeginPlay
  (CallFunction|GenerateAllRooms))

(event EventTick
  (params (DeltaSeconds :type Float%20%28single-precision%29)))

(fn GenerateRoom
  ;[1 1 1] Create X*Y Sized Room
  (bind _output_get (LocalVariables|SetSize (Math|Vector|MakeVector (Math|Conversions|ToFloat(Integer) (Math|Random|RandomIntegerinRange (Variables|Specifications|GetMinRoomSize) (Variables|Specifications|GetMaxRoomSize))) (Math|Conversions|ToFloat(Integer) (Math|Random|RandomIntegerinRange (Variables|Specifications|GetMinRoomSize) (Variables|Specifications|GetMaxRoomSize))) 0.0)))
  ;[1 1 1] Randomise Room Position within Map Size Grid
  (bind _output_get_2 (LocalVariables|SetPosition (Math|Vector|MakeVector (Math|Conversions|ToFloat(Integer) (Math|Random|RandomIntegerinRange 0 (- (Variables|Specifications|GetMaze%20Size) (Math|Float|Truncate (.X (Math|Vector|BreakVector _output_get)))))) (Math|Conversions|ToFloat(Integer) (Math|Random|RandomIntegerinRange 0 (- (Variables|Specifications|GetMaze%20Size) (Math|Float|Truncate (.Y (Math|Vector|BreakVector _output_get)))))) 0.0)))
  (return _output_get_2 (LocalVariables|GetSize)))

(fn CheckOverlap
  (params (RoomPosition :type Vector) (RoomSize :type Vector))
  (bind (_x _y) (Math|Vector|BreakVector RoomPosition))
  (bind (_x_2 _y_2) (Math|Vector|BreakVector RoomSize))
  ;[1 1 1] Check Overlap - Overlap Boolean Checkers not very clean but works for now
  ;;[1 1 1] Set Variables for New Room
  (LocalVariables|SetNewRoomXPos _x)
  (LocalVariables|SetNewRoomYPos _y)
  (LocalVariables|SetNewRoomXSize (+ _x _x_2))
  (LocalVariables|SetNewRoomYSize (+ _y _y_2))
  ;;[1 1 1] Set Variables for Old Room(s) - For Each Loop
  (for (_array_element _array_index) (Variables|Default|GetRoomPositions)
    (bind _output_get (LocalVariables|SetOldRoomXPos (.X (Math|Vector|BreakVector _array_element))))
    (bind _output_get_2 (LocalVariables|SetOldRoomYPos (.Y (Math|Vector|BreakVector _array_element))))
    (LocalVariables|SetOldRoomXSize (+ _output_get (.X (Math|Vector|BreakVector (Utilities|Array|Get(acopy) (Variables|Default|GetRoomSizes) _array_index)))))
    (LocalVariables|SetOldRoomYSize (+ _output_get_2 (.Y (Math|Vector|BreakVector (Utilities|Array|Get(acopy) (Variables|Default|GetRoomSizes) _array_index)))))
    (if (Math|Boolean|ORBoolean (Math|Boolean|ANDBoolean (<= (LocalVariables|GetNewRoomXPos) (LocalVariables|GetOldRoomXPos)) (<= (LocalVariables|GetNewRoomYPos) (LocalVariables|GetOldRoomYPos)) (>= (LocalVariables|GetNewRoomXSize) (LocalVariables|GetOldRoomXPos)) (>= (LocalVariables|GetNewRoomYSize) (LocalVariables|GetOldRoomYPos))) (Math|Boolean|ANDBoolean (<= (LocalVariables|GetOldRoomXPos) (LocalVariables|GetNewRoomXPos)) (<= (LocalVariables|GetOldRoomYPos) (LocalVariables|GetNewRoomYPos)) (>= (LocalVariables|GetOldRoomXSize) (LocalVariables|GetNewRoomXPos)) (>= (LocalVariables|GetOldRoomYSize) (LocalVariables|GetNewRoomYPos))) (Math|Boolean|ANDBoolean (>= (LocalVariables|GetOldRoomXPos) (LocalVariables|GetNewRoomXPos)) (<= (LocalVariables|GetOldRoomXPos) (LocalVariables|GetNewRoomXSize)) (>= (LocalVariables|GetOldRoomYSize) (LocalVariables|GetNewRoomYPos))) (Math|Boolean|ANDBoolean (>= (LocalVariables|GetNewRoomXPos) (LocalVariables|GetOldRoomXPos)) (<= (LocalVariables|GetNewRoomXPos) (LocalVariables|GetOldRoomXSize)) (>= (LocalVariables|GetNewRoomYPos) (LocalVariables|GetOldRoomYSize))) (Math|Boolean|ANDBoolean (>= (LocalVariables|GetOldRoomYPos) (LocalVariables|GetNewRoomYPos)) (<= (LocalVariables|GetOldRoomYPos) (LocalVariables|GetNewRoomYSize)) (>= (LocalVariables|GetOldRoomXSize) (LocalVariables|GetNewRoomXPos))) (Math|Boolean|ANDBoolean (>= (LocalVariables|GetNewRoomYPos) (LocalVariables|GetOldRoomYPos)) (<= (LocalVariables|GetNewRoomYPos) (LocalVariables|GetOldRoomYSize)) (>= (LocalVariables|GetNewRoomXSize) (LocalVariables|GetOldRoomXPos))))
      (return true)))
  (return false))

(fn GenerateAllRooms
  ;[1 1 1] Create Rooms as long as there is space
  (while (and (< (LocalVariables|GetCurrentRooms) (Variables|Specifications|GetMaxRooms)) (< (LocalVariables|GetFailCounter) (LocalVariables|GetMaxF)))
    (bind (_roomposition _roomsize) (CallFunction|GenerateRoom))
    ;[1 1 1] No Overlap - Room is Valid add to array
    (bind _overlap (CallFunction|CheckOverlap _roomposition _roomsize))
    (if _overlap
      (Math|Integer|IncrementInt (LocalVariables|GetFailCounter))
      (else
        (Utilities|Array|Add (Variables|Default|GetRoomPositions) _roomposition)
        (Utilities|Array|Add (Variables|Default|GetRoomSizes) _roomsize)
        (Math|Integer|IncrementInt (LocalVariables|GetCurrentRooms)
          (:%20%20
            (LocalVariables|SetFailCounter 0)))))))

(fn FindCenter
  ;[1 1 1] Find Center Points of each Room
  (for (_array_element _array_index) (Variables|Default|GetRoomPositions)
    (Utilities|Array|Add (Variables|Default|GetRoomCenterPoints) (Math|Vector|MakeVector (/ (+ (.X (Math|Vector|BreakVector _array_element)) (.X (Math|Vector|BreakVector (Utilities|Array|Get(acopy) (Variables|Default|GetRoomSizes) _array_index)))) 2.0) (/ (+ (.Y (Math|Vector|BreakVector _array_element)) (.Y (Math|Vector|BreakVector (Utilities|Array|Get(acopy) (Variables|Default|GetRoomSizes) _array_index)))) 2.0) (Math|Conversions|ToFloat(Integer) _array_index))))
  (return))

(fn KruskalMSTCorridors)