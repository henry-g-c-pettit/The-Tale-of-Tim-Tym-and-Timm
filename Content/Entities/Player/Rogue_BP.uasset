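; Rogue player character Blueprint that specializes a parent class with its own starting stats and first ability.
; BeginPlay initializes health, attack and speed through InitStats, and Tick continuously derives max walk speed from the Speed stat.
; The first ability doubles Speed and grants invincibility, and its end function reverses both.
; BasicAttack defers to the parent, passing a zero vector instead of the supplied position.
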(event EventBeginPlay
  (|CallParentFunction)
  (CallFunction|SetStats))

(event Collision|EventActorBeginOverlap
  (params (OtherActor :type Actor%20Object%20Reference))
  (|CallParentFunction OtherActor) ; This node is disabled and will not be called.\nDrag off pins to build functionality.
)

(event EventTick
  (params (DeltaSeconds :type Float%20%28single-precision%29))
  (|CallParentFunction DeltaSeconds)
  (Variables|/Script/Engine.CharacterMovementComponent|SetMaxWalkSpeed (Variables|Character|GetCharacterMovement) (* 20 (Variables|Default|GetSpeed))))

(fn ConstructionScript
  (|CallParentFunction))

(fn BasicAttack
  (params (Position :type Vector :default "0, 0, 0"))
  (bind _attack (|CallParentFunction "0, 0, 0"))
  (return _attack))

(fn EndFirstAbility
  (|CallParentFunction)
  (Variables|Default|SetSpeed (/ (Variables|Default|GetSpeed) 2.0))
  (Variables|Default|Setinvincible false))

(fn FirstAbility
  (|CallParentFunction)
  (Variables|Default|SetSpeed (* (Variables|Default|GetSpeed) 2.0))
  (Variables|Default|Setinvincible true))

(fn SetStats
  (CallFunction|InitStats (Variables|Default|GetstartHP) (Variables|Default|GetstartATK) (Variables|Default|GetstartSPD) 0.0))