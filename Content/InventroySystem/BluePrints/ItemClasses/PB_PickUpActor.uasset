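; Pickup actor that adds a set amount of an item class to the inventory of a TopDownCharacter that walks into it.
; Overlapping its Sphere component casts the other actor to TopDownCharacter and, if its inventory reference is valid, calls AddItem.
; On success the actor keeps any leftover amount for later pickup, or destroys itself when none remains.
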(event OnComponentBeginOverlap(Sphere)
  (params (OverlappedComponent :type Primitive%20Component%20Object%20Reference) (OtherActor :type Actor%20Object%20Reference) (OtherComp :type Primitive%20Component%20Object%20Reference) (OtherBodyIndex :type Integer) (bFromSweep :type Boolean) (SweepResult :type Hit%20Result%20Structure%20%28by%20ref%29))
  (bind _astop_down_character (Utilities|Casting|CastToTopDownCharacter OtherActor))
  (Utilities|IsValid (Variables|/Game/TopDownBP/Blueprints/TopDownCharacter.TopDownCharacter_C|GetInventoryRef _astop_down_character)
    (:Is%20Valid
      (bind (_success _rest) (Default|AddItem (Variables|/Game/TopDownBP/Blueprints/TopDownCharacter.TopDownCharacter_C|GetInventoryRef _astop_down_character) (Variables|Default|GetItemToAdd) (Variables|Default|GetAmmount)))
      (if _success
        (if (> _rest 0)
          (Variables|Default|SetAmmount _rest)
          (else
            (Actor|DestroyActor)))))))

(event EventBeginPlay)

(event Collision|EventActorBeginOverlap
  (params (OtherActor :type Actor%20Object%20Reference)))

(event EventTick
  (params (DeltaSeconds :type Float%20%28single-precision%29)))

(fn ConstructionScript)